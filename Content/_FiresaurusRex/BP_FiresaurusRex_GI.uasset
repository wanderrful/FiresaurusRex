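; Game instance for Firesaurus Rex that persists music volume and last level and manages background music.
; On Init it loads the save slot and copies its values into instance variables, or creates and saves a new save object if none exists.
; A write function copies those variables back to the save object and slot.
; A music function swaps the current 2D track for a new one at the saved volume, except in the MainMenu level.
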(event EventInit
  (bind _returnvalue (SaveGame|DoesSaveGameExist (Variables|SaveData|GetSaveSlotName)))
  (if _returnvalue
    (bind _returnvalue_2 (SaveGame|LoadGamefromSlot (Variables|SaveData|GetSaveSlotName)))
    (bind _asbp_firesaurus_rex_sg (Utilities|Casting|CastToBP_FiresaurusRex_SG _returnvalue_2))
    (Variables|SaveData|SetSaveGameRef _asbp_firesaurus_rex_sg)
    (CallFunction|FnReadSaveGameData)
    (else
      (bind _returnvalue_3 (SaveGame|CreateSaveGameObject "/Game/_FiresaurusRex/BP_FiresaurusRex_SG.BP_FiresaurusRex_SG_C"))
      (bind _output_get (Variables|SaveData|SetSaveGameRef _returnvalue_3))
      (SaveGame|SaveGametoSlot _output_get (Variables|SaveData|GetSaveSlotName)))))

(event EventShutdown)

(fn FnReadSaveGameData
  (bind _savegameref (Variables|SaveData|GetSaveGameRef))
  (Variables|Sound|SetMusicVolume (Variables|/Game/_FiresaurusRex/BP_FiresaurusRex_SG.BP_FiresaurusRex_SG_C|GetMusicVolume _savegameref))
  (Variables|Default|SetLastLevel (Variables|/Game/_FiresaurusRex/BP_FiresaurusRex_SG.BP_FiresaurusRex_SG_C|GetLastLevel _savegameref))
  (return))

(fn FnWriteSaveGameData
  (bind _savegameref (Variables|SaveData|GetSaveGameRef))
  (Utilities|IsValid _savegameref
    (:Is%20Valid
      (Variables|/Game/_FiresaurusRex/BP_FiresaurusRex_SG.BP_FiresaurusRex_SG_C|SetLastLevel _savegameref (Variables|Default|GetLastLevel))
      (Variables|/Game/_FiresaurusRex/BP_FiresaurusRex_SG.BP_FiresaurusRex_SG_C|SetMusicVolume _savegameref (Variables|Sound|GetMusicVolume))
      (SaveGame|SaveGametoSlot _savegameref (Variables|SaveData|GetSaveSlotName)))))

(fn FnPlayMusic
  (params (New%20Track :type Sound%20Base%20Object%20Reference))
  (bind _returnvalue (Game|GetCurrentLevelName true))
  (if (Utilities|Enum|NotEqual(Enum) _returnvalue "MainMenu")
    (Utilities|IsValid (Variables|Sound|GetMusicTheme)
      (:Is%20Valid
        (Audio|Components|Audio|Stop (Variables|Sound|GetMusicTheme)))
      (:Is%20Not%20Valid
        _))
    (bind _returnvalue_2 (Audio|SpawnSound2D New%20Track (Variables|Sound|GetMusicVolume)))
    (Variables|Sound|SetMusicTheme _returnvalue_2)
    (return)
    (else
      (return))))