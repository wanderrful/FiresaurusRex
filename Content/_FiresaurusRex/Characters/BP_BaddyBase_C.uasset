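; Base enemy Blueprint that hurts the player on contact and dies from any damage.
; Overlap between its HurtVolume and the player's capsule calls the hurt handler on BP_Player_C, passing itself.
; Death disables collision on mesh, hurt volume and capsule, while a timeline animates the mesh's XY and Z scale separately.
; When the timeline ends, it reports the death to BP_Game_GM and destroys itself.
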(event OnComponentBeginOverlap(HurtVolume)
  (params (OverlappedComponent :type Primitive%20Component%20Object%20Reference) (OtherActor :type Actor%20Object%20Reference) (OtherComp :type Primitive%20Component%20Object%20Reference) (OtherBodyIndex :type Integer) (bFromSweep :type Boolean) (SweepResult :type Hit%20Result%20Structure%20%28by%20ref%29))
  (bind _asbp_player_c (Utilities|Casting|CastToBP_Player_C OtherActor))
  (Utilities|Casting|CastToCapsuleComponent OtherComp)
  (Default|EhonWasHurt _asbp_player_c self))

(event Custom|eh_OnWasKilled
  (bind _mesh (Variables|Character|GetMesh))
  (bind _returnvalue (Transformation|GetWorldTransform _mesh))
  (for _array_element (Utilities|Array|MakeArray (Variables|Character|GetMesh) (Variables|Default|GetHurtVolume) (Variables|Default|GetCapsuleComponent))
    (Collision|SetCollisionEnabled (.AsPrimitive%20Component (Utilities|Casting|CastToPrimitiveComponent _array_element)) "NoCollision")
    (if (not (Audio|Components|Audio|IsPlaying (Variables|Default|GetTimeline_0)))
      (bind (_direction _scale_z _scale_xy) (Timeline|Timeline_0 PlayFromStart)
        (:Update
          (Transformation|SetWorldTransform _mesh (Math|Transform|MakeTransform (.location _returnvalue) (.rotation _returnvalue) (Math|Vector|MakeVector _scale_xy _scale_xy _scale_z)) false false))
        (:Finished
          (bind _asbp_game_gm (Utilities|Casting|CastToBP_Game_GM (Game|GetGameMode)))
          (Default|CallEdonDeath _asbp_game_gm self)
          (Actor|DestroyActor))))))

(event Game|Damage|EventAnyDamage
  (params (Damage :type Float%20%28single-precision%29) (DamageType :type Damage%20Type%20Object%20Reference) (InstigatedBy :type Controller%20Object%20Reference) (DamageCauser :type Actor%20Object%20Reference))
  (CallFunction|EhonWasKilled))

(fn ConstructionScript)