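; BP_FireWhelp is a fire whelp character that hops on a repeating timer and varies its appearance per instance.
; The construction script randomly picks one of two materials, tinting the three point lights blue for the second.
; It also randomly swaps in the Whomp mesh with its animation Blueprint and randomizes scale independently on each axis.
; On BeginPlay, a looping timer with a randomly chosen, fixed interval calls Jump.
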(event Custom|CustomEvent_0
  (Character|Jump))

(event EventBeginPlay
  (Utilities|Time|SetTimerbyEvent (delegate Custom|CustomEvent_0) (Math|Random|RandomFloatinRange 2.0 5.0) true))

(fn ConstructionScript
  (bind _returnvalue (Math|Random|RandomFloatinRange 0.6 1.05))
  (bind _mesh (Variables|Character|GetMesh))
  (bind _mesh_2 (Variables|Character|GetMesh))
  (|CallParentFunction)
  (Utilities|FlowControl|Sequence
    (:then_0
      (if (Math|Random|RandomBool)
        (Rendering|Material|SetMaterial _mesh_2 0 "/Game/_FiresaurusRex/Characters/firewhelps/red/lambert6.lambert6")
        (else
          (Rendering|Material|SetMaterial _mesh_2 0 "/Game/_FiresaurusRex/Characters/firewhelps/blue/lambert8.lambert8")
          (for _array_element (Utilities|Array|MakeArray (Variables|Default|GetPointLight) (Variables|Default|GetPointLight1) (Variables|Default|GetPointLight2))
            (Rendering|Components|Light|SetLightColor _array_element "(R=0.119792,G=0.545756,B=1.000000,A=1.000000)" true)))))
    (:then_1
      (if (Math|Random|RandomBool)
        (Class|SkinnedMeshComponent|SetSkeletalMesh _mesh "/Game/_FiresaurusRex/animations/flamewhelps/whomp/whomp.whomp" true)
        (Components|SkeletalMesh|SetAnimInstanceClass _mesh "/Game/_FiresaurusRex/animations/flamewhelps/whomp/ABP_Whomp.ABP_Whomp_C")))
    (:then_2
      (Transformation|SetActorScale3D (Math|Vector|MakeVector _returnvalue _returnvalue _returnvalue)))))