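; BP_Base_AIC is a base AI controller that runs the BT_FireWhelp behavior tree on BeginPlay and tracks the player through AI perception.
; On each perception update, it writes the first BP_Player found among the updated actors to the Blackboard's PlayerKey.
; It then clears that key if the stored actor is absent from the currently sight-perceived actors, so the Blackboard holds the player only while seen.
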(event OnPerceptionUpdated(AIPerception)
  (params (UpdatedActors :type Array%20of%20Actor%20Object%20References))
  (bind _blackboard (Variables|Default|GetBlackboard))
  (bind _playerkey (Variables|Default|GetPlayerKey))
  (bind _array_element (Utilities|Array|ForEachLoopwithBreak UpdatedActors :!label _label)
    (:LoopBody
      (bind _asbp_player_c (Utilities|Casting|CastToBP_Player_C _array_element))
      (AI|Components|Blackboard|SetValueasObject (Variables|Default|GetBlackboard) (Variables|Default|GetPlayerKey) _asbp_player_c)
      (goto _label Break))
    (:Completed
      ;[1 1 1] If the player isn't being perceived, reset the Blackboard key
      (bind _asactor (Utilities|Casting|CastToActor (AI|Components|Blackboard|GetValueasObject _blackboard _playerkey))
        (:then
          (if (not (Utilities|Array|ContainsItem (Class|AIPerceptionComponent|GetCurrentlyPerceivedActors (Variables|Default|GetAIPerception) "/Script/AIModule.AISense_Sight") _asactor))
            (AI|Components|Blackboard|SetValueasObject _blackboard _playerkey 0 :!label _label_2)))
        (:CastFailed
          (goto _label_2))))))

(event EventBeginPlay
  (AI|RunBehaviorTree "/Game/_FiresaurusRex/Core/AI/BT_FireWhelp.BT_FireWhelp"))

(fn ConstructionScript)