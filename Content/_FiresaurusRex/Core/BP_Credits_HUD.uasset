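; BP_Credits_HUD is the HUD Blueprint that displays the credits screen.
; On BeginPlay it creates the WB_Credits widget, adds it to the viewport, switches input to UI-only focused on it and shows the mouse cursor.
; On EndPlay it removes the widget, keeps the cursor visible only if the game is paused, and returns focus to the game viewport.
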(event EventBeginPlay
  (bind _returnvalue (Game|Player|GetOwningPlayerController))
  (bind _returnvalue_2 (UserInterface|CreateWidget "/Game/_FiresaurusRex/UI/WB_Credits.WB_Credits_C" _returnvalue))
  (bind _output_get (Variables|Default|SetUI_Credits _returnvalue_2))
  (UserInterface|Viewport|AddtoViewport _output_get 0)
  (Input|SetInputModeUIOnly _returnvalue (Variables|Default|GetUI_Credits) "DoNotLock")
  (Variables|/Script/Engine.PlayerController|SetbShowMouseCursor (Game|Player|GetOwningPlayerController) true))

(event EventEndPlay
  (params (EndPlayReason :type EEndPlayReason%20Enum :default "Destroyed"))
  (Widget|RemovefromParent (Variables|Default|GetUI_Credits))
  (Variables|/Script/Engine.PlayerController|SetbShowMouseCursor (Game|Player|GetOwningPlayerController) (Game|IsGamePaused))
  (Class|WidgetBlueprintLibrary|SetFocustoGameViewport))

(fn ConstructionScript)