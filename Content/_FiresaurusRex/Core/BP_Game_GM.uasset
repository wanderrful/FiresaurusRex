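; Game mode for Firesaurus Rex that handles level progression and player pawn spawning.
; On BeginPlay it saves recognized jam level names to the game instance as LastLevel and binds death and progression dispatchers.
; Baddy deaths are counted, triggering progression at set totals in JamLevel_02 and JamLevel_04.
; Progression runs a global time dilation timeline before opening the next level; the spawn override uses a no-gear plush pawn in JamLevel.
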(event Custom|ed_ProgressToNextLevel_Event
  (params (NextLevel :type Name))
  (if (not (Audio|Components|Audio|IsPlaying (Variables|Default|GetTimeline_0)))
    (bind _timedilation (Timeline|Timeline_0 PlayFromStart)
      (:Update
        (Utilities|Time|SetGlobalTimeDilation _timedilation))
      (:Finished
        (Game|OpenLevel(byName) NextLevel)))))

(event Custom|ed_OnDeath_Event
  (params (PawnThatDied :type Pawn%20Object%20Reference))
  (bind _deathcount (Variables|Default|GetDeathCount))
  (Utilities|Casting|CastToBP_BaddyBase_C PawnThatDied)
  (Math|Integer|IncrementInt (Variables|Default|GetDeathCount)
    (:%20%20
      (bind _returnvalue (Game|GetCurrentLevelName true))
      (switch string _returnvalue
        (:JamLevel_02
          (if (>= _deathcount 12)
            (Default|CallEdProgresstoNextLevel "JamLevel_03")))
        (:JamLevel_04
          (if (>= _deathcount 25)
            (Default|CallEdProgresstoNextLevel "EndingLevel")))))))

(event EventBeginPlay
  (Utilities|FlowControl|Sequence
    (:then_0
      (bind _returnvalue (Game|GetCurrentLevelName true))
      (if (Utilities|Array|ContainsItem (Utilities|Array|MakeArray "JamLevel" "JamLevel_02" "JamLevel_03" "JamLevel_04") _returnvalue)
        (bind _asbp_firesaurus_rex_gi (Utilities|Casting|CastToBP_FiresaurusRex_GI (Game|GetGameInstance)))
        (Variables|/Game/_FiresaurusRex/BP_FiresaurusRex_GI.BP_FiresaurusRex_GI_C|SetLastLevel _asbp_firesaurus_rex_gi _returnvalue)))
    (:then_1
      (EventDispatchers|BindEventtoEdProgresstoNextLevel (delegate Custom|ed_ProgressToNextLevel_Event))
      (EventDispatchers|BindEventtoEdonDeath (delegate Custom|ed_OnDeath_Event)))))

(fn ConstructionScript)

(fn SpawnDefaultPawnfor
  (params (NewPlayer :type Controller%20Object%20Reference) (StartSpot :type Actor%20Object%20Reference))
  (bind _returnvalue (Transformation|GetActorTransform StartSpot))
  (bind _returnvalue_2 (Game|GetCurrentLevelName true))
  (if (Utilities|Enum|Equal(Enum) _returnvalue_2 "JamLevel")
    (bind _returnvalue_3 (Game|SpawnActorfromClass "/Game/_FiresaurusRex/Characters/BP_PlayerPlush_NoGear.BP_PlayerPlush_NoGear_C" _returnvalue "AdjustIfPossibleButAlwaysSpawn" NewPlayer 0))
    (return _returnvalue_3)
    (else
      (bind _returnvalue_4 (Class|GameModeBase|GetDefaultPawnClassforController NewPlayer))
      (bind _aspawn (Utilities|Casting|CastToPawnClass _returnvalue_4))
      (bind _returnvalue_5 (Game|SpawnActorfromClass _aspawn _returnvalue "AdjustIfPossibleButAlwaysSpawn" NewPlayer 0))
      (return _returnvalue_5))))