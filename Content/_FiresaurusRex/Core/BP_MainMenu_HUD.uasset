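; Main menu HUD that puts the WB_MainMenu widget on screen for the owning player.
; On BeginPlay it creates the widget, stores it and adds it to the viewport, then shows the mouse cursor and sets Game and UI input mode focused on the menu.
; On EndPlay it removes the widget from its parent.
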(event EventBeginPlay
  (bind _returnvalue (Game|Player|GetOwningPlayerController))
  (CallFunction|FnInitWidgets)
  (Variables|/Script/Engine.PlayerController|SetbShowMouseCursor _returnvalue true)
  (Input|SetInputModeGameandUI _returnvalue (Variables|Default|GetUI_MainMenu) "DoNotLock" false))

(event EventEndPlay
  (params (EndPlayReason :type EEndPlayReason%20Enum :default "Destroyed"))
  (Widget|RemovefromParent (Variables|Default|GetUI_MainMenu)))

(fn ConstructionScript)

(fn FnInitWidgets
  (bind _returnvalue (UserInterface|CreateWidget "/Game/_FiresaurusRex/UI/WB_MainMenu.WB_MainMenu_C" (Game|Player|GetOwningPlayerController)))
  (bind _output_get (Variables|Default|SetUI_MainMenu _returnvalue))
  (UserInterface|Viewport|AddtoViewport _output_get 0)
  (return))