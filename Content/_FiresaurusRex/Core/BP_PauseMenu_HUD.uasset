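; Pause menu HUD class that pauses the game and shows the WB_PauseMenu widget while it is active.
; On BeginPlay it creates the widget, switches input to UI only and shows the mouse cursor.
; On EndPlay it removes the widget, returns focus to the viewport, hides the cursor and sets the player's HUD to BP_Game_HUD.
; It does not unpause the game itself.
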(event EventBeginPlay
  (bind _returnvalue (Game|Player|GetOwningPlayerController))
  (Game|SetGamePaused true)
  (bind _returnvalue_2 (UserInterface|CreateWidget "/Game/_FiresaurusRex/UI/WB_PauseMenu.WB_PauseMenu_C" _returnvalue))
  (bind _output_get (Variables|Default|SetUI_Pause _returnvalue_2))
  (UserInterface|Viewport|AddtoViewport _output_get 0)
  (Input|SetInputModeUIOnly _returnvalue (Variables|Default|GetUI_Pause) "DoNotLock")
  (Variables|/Script/Engine.PlayerController|SetbShowMouseCursor _returnvalue true))

(event EventEndPlay
  (params (EndPlayReason :type EEndPlayReason%20Enum :default "Destroyed"))
  (Class|WidgetBlueprintLibrary|SetFocustoGameViewport)
  (Widget|RemovefromParent (Variables|Default|GetUI_Pause))
  (Variables|/Script/Engine.PlayerController|SetbShowMouseCursor (Game|Player|GetOwningPlayerController) false)
  (Class|PlayerController|ClientSetHUD (Game|Player|GetOwningPlayerController) "/Game/_FiresaurusRex/Core/BP_Game_HUD.BP_Game_HUD_C"))

(fn ConstructionScript)