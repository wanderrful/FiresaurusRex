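; BP_EnemySpawner is a placed actor that spawns a configured enemy class at its own transform.
; After an initial delay, its Type selects endless mode, which spawns on a looping timer, or wave mode, which spawns whenever the BP_Game_GM game mode broadcasts its wave-complete event.
; Spawns adjust position to avoid collisions and are skipped if no clear spot is found.
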(event Custom|CustomEvent_0
  (CallFunction|FnSpawnBaddy))

(event Custom|CustomEvent_1
  (CallFunction|FnSpawnBaddy))

(event EventBeginPlay
  (Utilities|FlowControl|Delay (Variables|Default|GetInitialDelay))
  (switch Utilities|FlowControl|Switch|SwitchonESpawnerType (Variables|Default|GetType)
    (:NewEnumerator0
      (Utilities|Time|SetTimerbyEvent (delegate Custom|CustomEvent_0) (Variables|Default|GetSpawnInterval) true))
    (:NewEnumerator1
      (bind _asbp_game_gm (Utilities|Casting|CastToBP_Game_GM (Game|GetGameMode)))
      (EventDispatchers|BindEventtoEdonWaveComplete _asbp_game_gm (delegate Custom|CustomEvent_1)))))

(fn ConstructionScript)

(fn FnSpawnBaddy
  (Game|SpawnActorfromClass (Variables|Default|GetBaddyToSpawn) (Transformation|GetActorTransform) "AdjustIfPossibleButDontSpawnIfColliding" 0 0)
  (return))